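; BP_Player is the player-controlled pawn, handling basic movement and camera look through Enhanced Input.
; On possession by a PlayerController, it adds the IMC_Base mapping context to the local player subsystem.
; IA_Look feeds controller yaw and pitch, while IA_PlayerMove applies scaled movement input along the actor's forward (X) and right (Y) vectors.
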(event `self.ReceivePossessed`
  (params (NewController :type "Controller Object Reference"))
  (bind _asplayer_controller (cast `PlayerController` NewController))
  (`EnhancedInputSubsystemInterface.AddMappingContext` (pcsubsystem `EnhancedInputLocalPlayerSubsystem` _asplayer_controller) "/Game/Custom/Character/IMC_Base.IMC_Base" 0 (struct)))

(event `EnhancedInput|/Game/ThirdPerson/Input/Actions/IA_Look`
  (params (ActionValue :type "Vector2D Structure") (ElapsedSeconds :type "Float (double-precision)") (TriggeredSeconds :type "Float (double-precision)") (InputAction :type "InputAction Object Reference" :default "/Game/ThirdPerson/Input/Actions/IA_Look.IA_Look"))
  ; Comment
  (:`Triggered`
    (`self.AddControllerYawInput` ActionValue_X)
    (`self.AddControllerPitchInput` ActionValue_Y)))

(event `EnhancedInput|/Game/Custom/Character/IA_PlayerMove`
  (params (ActionValue :type "Vector2D Structure") (ElapsedSeconds :type "Float (double-precision)") (TriggeredSeconds :type "Float (double-precision)") (InputAction :type "InputAction Object Reference" :default "/Game/Custom/Character/IA_PlayerMove.IA_PlayerMove"))
  (:`Triggered`
    (`self.AddMovementInput` (`self.GetActorRightVector`) (* ActionValue_Y 1000.0))
    (`self.AddMovementInput` (`self.GetActorForwardVector`) (* ActionValue_X 1000.0))))

(fn `UserConstructionScript`)
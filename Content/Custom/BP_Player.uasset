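; Player pawn Blueprint that handles first-hand look and movement input and displays its current health.
; On possession by a player controller it adds the IMC_PlayerInputs Enhanced Input mapping context.
; IA_Look drives controller yaw and pitch, while IA_Move adds movement along the actor's forward and right vectors.
; Tick writes CurrentHP to the HP text every frame.
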(event `self.ReceivePossessed`
  (params (NewController :type "Controller Object Reference"))
  (bind _asplayer_controller (cast `PlayerController` NewController))
  (`EnhancedInputSubsystemInterface.AddMappingContext` (pcsubsystem `EnhancedInputLocalPlayerSubsystem` _asplayer_controller) "/Game/Custom/InputAction/IMC_PlayerInputs.IMC_PlayerInputs" 0 (struct)))

(event `EnhancedInput|/Game/ThirdPerson/Input/Actions/IA_Look`
  (params (ActionValue :type "Vector2D Structure") (ElapsedSeconds :type "Float (double-precision)") (TriggeredSeconds :type "Float (double-precision)") (InputAction :type "InputAction Object Reference" :default "/Game/ThirdPerson/Input/Actions/IA_Look.IA_Look"))
  ; Comment
  (:`Triggered`
    (`self.AddControllerYawInput` ActionValue_X)
    (`self.AddControllerPitchInput` ActionValue_Y)))

(event `EnhancedInput|/Game/Custom/InputAction/IA_Move`
  (params (ActionValue :type "Vector2D Structure") (ElapsedSeconds :type "Float (double-precision)") (TriggeredSeconds :type "Float (double-precision)") (InputAction :type "InputAction Object Reference" :default "/Game/Custom/InputAction/IA_Move.IA_Move"))
  (:`Triggered`
    (`self.AddMovementInput` (`self.GetActorRightVector`) (* ActionValue_Y 1000.0))
    (`self.AddMovementInput` (`self.GetActorForwardVector`) (* ActionValue_X 1000.0))))

(event `self.ReceiveTick`
  (params (DeltaSeconds :type "Float (single-precision)"))
  (`TextRenderComponent.K2_SetText` (`self.HP`) (`KismetTextLibrary.Conv_DoubleToText` (`self.CurrentHP`) "HalfToEven")))

(fn `UserConstructionScript`)